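; Enemy spawner actor that populates the level with named AI enemies when play begins.
; It gathers every BP_EnemySpawnPoint and gives each a weighted random chance to spawn a BP_AiMoveTo at that point's transform.
; Each spawned AI gets its AIName text set from a randomly indexed entry in the AINames array.
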(event EventBeginPlay
  (bind _ai_names (Variables|Default|GetAI_Names))
  (Development|PrintString "enemy spawner is active")
  (bind _outactors (Actor|GetAllActorsOfClass "/Game/Blueprints/BP_EnemySpawnPoint.BP_EnemySpawnPoint_C"))
  (for _array_element _outactors
    (if (Math|Random|RandomBoolwithWeight 0.45)
      (bind _returnvalue (Game|SpawnActorfromClass "/Game/AI_Blueprints/BP_AiMoveTo.BP_AiMoveTo_C" (Transformation|GetActorTransform _array_element) "Undefined" "MultiplyWithRoot" 0 0))
      (Rendering|Components|TextRender|SetText (Variables|/Game/AI_Blueprints/BP_AiMoveTo.BP_AiMoveTo_C|GetAI%20Name _returnvalue) (Utilities|Array|Get(acopy) _ai_names (Math|Float|Truncate (Math|Random|RandomFloatinRange 0.0 (Math|Conversions|ToFloat(Integer) (Utilities|Array|Length _ai_names)))))))))

(event Collision|EventActorBeginOverlap
  (params (OtherActor :type Actor%20Object%20Reference)))

(event EventTick
  (params (DeltaSeconds :type Float%20%28single-precision%29)))

(fn ConstructionScript)