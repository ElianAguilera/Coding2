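; BP_MachineGun is a machine gun weapon actor that can be picked up, used and dropped.
; PickUp prints a message, snaps the gun to the given skeletal mesh's hand_r socket and disables the Cube's collision.
; UsePrimary is a placeholder that only prints firing text.
; Drop detaches the gun, re-runs an attach with no parent set, briefly simulates Cube physics with collision restored, then stops physics and calls Reset.
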(event EventBeginPlay)

(event Collision|EventActorBeginOverlap
  (params (OtherActor :type Actor%20Object%20Reference)))

(event EventTick
  (params (DeltaSeconds :type Float%20%28single-precision%29)))

(event EventPickUp
  (params (SkeletalMesh :type Skeletal%20Mesh%20Component%20Object%20Reference))
  ;[0.15 0.15 0.15 0.5] PickupFunction
  (Development|PrintText (Utilities|Text|FormatText "{name} is getting picked up and attached to {mesh}" (Utilities|String|MakeLiteralString "Machine Gun") SkeletalMesh) true true "(R=0.286653,G=0.278908,B=1.000000,A=1.000000)" 5.0)
  (Transformation|AttachComponentToComponent SkeletalMesh "hand_r" "SnapToTarget" "SnapToTarget" "KeepRelative" true)
  (Collision|SetCollisionEnabled (Variables|Default|GetCube) "NoCollision"))

(event EventUsePrimary
  (Development|PrintText "Pew Pew Pew"))

(event EventDrop
  (bind _cube (Variables|Default|GetCube))
  (Transformation|DetachFromActor "KeepWorld" "KeepWorld" "KeepRelative")
  (Transformation|AttachComponentToComponent 0 "None" "KeepWorld" "KeepWorld" "KeepRelative" true)
  (Physics|SetSimulatePhysics _cube true)
  (Collision|SetCollisionEnabled _cube "QueryAndPhysics")
  (Utilities|FlowControl|Delay 1.0)
  (Physics|SetSimulatePhysics (Variables|Default|GetCube) false)
  (Class|TypedElementListLibrary|Reset))

(fn ConstructionScript)