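; Game mode that handles saving and loading of player stats and per-level coin state.
; On BeginPlay it loads or creates two save objects: SG_PlayerStats in a fixed slot and SG_LevelState in a slot named after the current level.
; Loading copies Stamina to the third-person character and calls AlreadyCollected on each valid saved coin reference.
; Save events write the held objects to their slots without gathering values themselves.
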(event Custom|Load%20Player%20Stats
  (bind _returnvalue (SaveGame|DoesSaveGameExist "PlayerSave"))
  (if _returnvalue
    (bind _returnvalue_2 (SaveGame|LoadGamefromSlot "PlayerSave"))
    (bind _assg_player_stats (Utilities|Casting|CastToSG_PlayerStats _returnvalue_2))
    (Variables|Default|SetSG_PlayerStats _assg_player_stats)
    (bind _asbp_third_person_character (Utilities|Casting|CastToBP_ThirdPersonCharacter (Game|GetPlayerCharacter 0)))
    (Variables|/Game/ThirdPerson/Blueprints/BP_ThirdPersonCharacter.BP_ThirdPersonCharacter_C|SetStamina _asbp_third_person_character (Variables|/Game/Blueprints/SavingLoading/SG_PlayerStats.SG_PlayerStats_C|GetStamina (Variables|Default|GetSG_PlayerStats)))
    (Development|PrintString "PlayerStats have been loaded" true true "(R=1.000000,G=0.684040,B=0.100115,A=1.000000)")
    (else
      (bind _returnvalue_3 (SaveGame|CreateSaveGameObject "/Game/Blueprints/SavingLoading/SG_PlayerStats.SG_PlayerStats_C"))
      (Variables|Default|SetSG_PlayerStats _returnvalue_3) ; Set this variable so that the player can edit these values
    )))

(event Custom|Save%20Player%20Stats
  (bind _returnvalue (SaveGame|SaveGametoSlot (Variables|Default|GetSG_PlayerStats) "PlayerSave"))
  (if _returnvalue
    (Development|PrintText "Player Stats Written to Save Game File" true true "(R=1.000000,G=0.501650,B=0.001757,A=1.000000)" 5.0)
    (else
      (Development|PrintText "Player Stats could not be written to Save Game File" true true "(R=1.000000,G=0.001721,B=0.233171,A=1.000000)" 5.0))))

(event Custom|SaveLevelState
  (bind _returnvalue (Game|GetCurrentLevelName true))
  (bind _returnvalue_2 (SaveGame|SaveGametoSlot (Variables|Default|GetSG_LevelState) _returnvalue))
  (if _returnvalue_2
    (Development|PrintText "Level State written to game file")
    (else
      (Development|PrintText "Player Stats could not be written to Save Game File" true true "(R=1.000000,G=0.001721,B=0.233171,A=1.000000)" 5.0))))

(event Custom|Load%20Level%20State
  (bind _returnvalue (Game|GetCurrentLevelName true))
  (bind _returnvalue_2 (SaveGame|DoesSaveGameExist _returnvalue))
  (if _returnvalue_2
    (bind _returnvalue_3 (SaveGame|LoadGamefromSlot _returnvalue))
    (bind _assg_level_state (Utilities|Casting|CastToSG_LevelState _returnvalue_3))
    (bind _output_get (Variables|Default|SetSG_LevelState _assg_level_state))
    (for _array_element (Variables|/Game/Blueprints/SavingLoading/SG_LevelState.SG_LevelState_C|GetCollectedCoins _output_get)
      (Utilities|IsValid _array_element
        (:Is%20Valid
          (Default|AlreadyCollected _array_element))
        (:Is%20Not%20Valid
          (Development|PrintText "Coins are not being Loaded"))))
    (Development|PrintText "Coin State Loaded." true true "(R=0.249045,G=0.000000,B=1.000000,A=1.000000)" 5.0)
    (else
      (bind _returnvalue_4 (SaveGame|CreateSaveGameObject "/Game/Blueprints/SavingLoading/SG_LevelState.SG_LevelState_C"))
      (Variables|Default|SetSG_LevelState _returnvalue_4))))

(event EventBeginPlay
  (Development|PrintString "Loading the SavLoad Game Mode" true true "(R=1.000000,G=0.461384,B=0.102434,A=1.000000)" 5.0)
  (CallFunction|LoadPlayerStats)
  (CallFunction|LoadLevelState))

(event EventTick
  (params (DeltaSeconds :type Float%20%28single-precision%29)))

(fn ConstructionScript)