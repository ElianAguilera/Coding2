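; BP_ElementalBarrier is an elemental barrier actor that checks whether the third-person character touching it is immune to its element.
; On BeginPlay it switches on ElementalType to label its TextRender as a Fire, Water, Grass or Dark barrier.
; When the Cube is overlapped, it compares the character's ElementalImmunity to that type and only prints a pass-through message on a match, with no blocking or damage logic in the graph.
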(event OnComponentBeginOverlap(Cube)
  (params (OverlappedComponent :type Primitive%20Component%20Object%20Reference) (OtherActor :type Actor%20Object%20Reference) (OtherComp :type Primitive%20Component%20Object%20Reference) (OtherBodyIndex :type Integer) (bFromSweep :type Boolean) (SweepResult :type Hit%20Result%20Structure%20%28by%20ref%29))
  (bind _asbp_third_person_character (Utilities|Casting|CastToBP_ThirdPersonCharacter OtherActor))
  (if (Utilities|Enum|Equal(Enum) (Variables|/Game/ThirdPerson/Blueprints/BP_ThirdPersonCharacter.BP_ThirdPersonCharacter_C|GetElementalImmunity _asbp_third_person_character) (Variables|Default|GetElementalType))
    (Development|PrintString "Barrier Went Through!")))

(event EventBeginPlay
  (switch Utilities|FlowControl|Switch|SwitchonBP_ElementalTypes (Variables|Default|GetElementalType)
    (:NewEnumerator0
      (Rendering|Components|TextRender|SetText (Variables|Default|GetTextRender) (Utilities|Text|MakeLiteralText "Barrier of Fire")))
    (:NewEnumerator1
      (Rendering|Components|TextRender|SetText (Variables|Default|GetTextRender) (Utilities|Text|MakeLiteralText "Barrier of Water")))
    (:NewEnumerator2
      (Rendering|Components|TextRender|SetText (Variables|Default|GetTextRender) (Utilities|Text|MakeLiteralText "Barrier of Grass")))
    (:NewEnumerator3
      (Rendering|Components|TextRender|SetText (Variables|Default|GetTextRender) (Utilities|Text|MakeLiteralText "Barrier of Dark")))))

(fn ConstructionScript)