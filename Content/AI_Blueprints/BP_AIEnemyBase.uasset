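; Base AI enemy character that supplies attack, aggro, speed, damage and patrol-point functions.
; Attack plays a montage and calls CallAttackFinished on completion or interruption, while aggro toggles a flag and swaps the mesh material.
; Point damage reduces Health and, at zero or below, triggers a ragdoll with a radial impulse from just below the hit location.
; Patrol locations come from indexed points on the PatrolRoute spline.
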(event Custom|Attack
  (Development|PrintString "Attacking Player")
  (Animation|Montage|PlayMontage (Variables|Character|GetMesh) "/Game/CloseCombatAnimSet/EnemyBaseAttack.EnemyBaseAttack"
    (:OnCompleted
      _)
    (:OnInterrupted
      _))
  (Default|CallAttackFinished))

(event Custom|GetAggro
  (Rendering|Material|SetMaterial (Variables|Character|GetMesh) 0 "/Engine/VREditor/LaserPointer/LaserPointerMaterial.LaserPointerMaterial")
  (Variables|Default|SetAggroed true))

(event Custom|LoseAggro
  (Rendering|Material|SetMaterial (Variables|Character|GetMesh) 0 (Variables|Default|GetOriginal%20Material))
  (Variables|Default|SetAggroed false))

(event Custom|setSpeed
  (params (New%20Speed :type Float%20%28single-precision%29))
  (Variables|/Script/Engine.CharacterMovementComponent|SetMaxWalkSpeed (Variables|Character|GetCharacterMovement) New%20Speed))

(event Custom|Ragdoll
  (params (Origin :type Vector))
  (bind _mesh (Variables|Character|GetMesh))
  (Physics|SetSimulatePhysics _mesh true)
  (Physics|AddRadialForce _mesh (+ Origin "0.000000,0.000000,-50.000000") 5e+02 5e+04 "RIF_Constant" true)
  (Pawn|Components|CharacterMovement|DisableMovement (Variables|Character|GetCharacterMovement)))

(event EventBeginPlay
  (Variables|Default|SetOriginal%20Material (Rendering|Material|GetMaterial (Variables|Character|GetMesh) 0)))

(event Game|Damage|EventAnyDamage
  (params (Damage :type Float%20%28single-precision%29) (DamageType :type Damage%20Type%20Object%20Reference) (InstigatedBy :type Controller%20Object%20Reference) (DamageCauser :type Actor%20Object%20Reference)))

(event Game|Damage|EventPointDamage
  (params (Damage :type Float%20%28single-precision%29) (DamageType :type Damage%20Type%20Object%20Reference) (HitLocation :type Vector :default "0, 0, 0") (HitNormal :type Vector :default "0, 0, 0") (HitComponent :type Primitive%20Component%20Object%20Reference) (BoneName :type Name :default "None") (ShotFromDirection :type Vector :default "0, 0, 0") (InstigatedBy :type Controller%20Object%20Reference) (DamageCauser :type Actor%20Object%20Reference) (HitInfo :type Hit%20Result%20Structure%20%28by%20ref%29))
  (Development|PrintText (Utilities|Text|FormatText "{instigator} damaged us for {dmg} damage!" InstigatedBy Damage) true true "(R=1.000000,G=0.005041,B=0.000000,A=1.000000)" 5.0)
  (bind _output_get (Variables|Default|SetHealth (- (Variables|Default|GetHealth) Damage)))
  (if (<= _output_get 0.0)
    (Development|PrintString "We are dead!")
    (CallFunction|Ragdoll HitLocation)))

(fn ConstructionScript)

(fn GetNextPatrolPointLocation
  (return (Spline|GetLocationatSplinePoint (Variables|/Game/AI_Blueprints/BP_PatrolRoute.BP_PatrolRoute_C|GetSpline (Variables|Default|GetPatrolRoute)) (Variables|Default|GetPatrol%20Point%20Index) "World")))